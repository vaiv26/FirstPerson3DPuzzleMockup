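; BP_PuzzleFirstCharacter is a character Blueprint that moves its camera spring arm between its default placement and a puzzle view.
; BeginPlay caches the SpringArm's relative transform as OriginalLocation.
; Each PlaySequence call alternates through a FlipFlop, easing the arm's location and rotation to PuzzleTransform or back to the cached transform with MoveComponentTo, returning faster than it moves out.
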(event EventBeginPlay
  (Variables|Default|SetOriginalLocation (Transformation|GetRelativeTransform (Variables|Default|GetSpringArm))))

(event Collision|EventActorBeginOverlap
  (params (OtherActor :type Actor%20Object%20Reference)))

(event EventTick
  (params (DeltaSeconds :type Float%20%28single-precision%29)))

(event EventPlaySequence
  (bind _puzzletransform (Variables|Default|GetPuzzleTransform))
  (bind _originallocation (Variables|Default|GetOriginalLocation))
  (bind (_location _rotation) (Math|Transform|BreakTransform _puzzletransform))
  (bind (_location_2 _rotation_2) (Math|Transform|BreakTransform _originallocation))
  (Utilities|FlowControl|FlipFlop
    (:A
      (Components|MoveComponentTo (Variables|Default|GetSpringArm) _location _rotation true true 6.0 false))
    (:B
      (Components|MoveComponentTo (Variables|Default|GetSpringArm) _location_2 _rotation_2 true true 4.0 false))))

(fn ConstructionScript)